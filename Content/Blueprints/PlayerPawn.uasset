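; Player pawn that moves tile to tile on a grid, turning to face the pressed direction.
; Directional inputs, ignored while a target tile is set, look up the current tile's neighbour and trigger move and rotate events.
; Timelines lerp location and rotation, entering only tiles of one type.
; On arrival, GetNextTile on the tile just left can chain another move automatically.
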(event Custom|MoveToTile
  (params (Destination :type Tile%20Object%20Reference))
  (if (Utilities|Enum|Equal(Enum) (Variables|/Game/Blueprints/Tile.Tile_C|GetTileType Destination) "NewEnumerator0")
    (Variables|Default|SetTargetTile Destination)
    (bind _moveprogress (Timeline|MoveTimeline PlayFromStart)
      (:Update
        (Transformation|SetActorLocation (Math|Vector|Lerp(Vector) (Transformation|GetActorLocation (Variables|Default|GetCurrentTile)) (Transformation|GetActorLocation (Variables|Default|GetTargetTile)) _moveprogress) false false))
      (:Finished
        (Variables|Default|SetTemp (Variables|Default|GetCurrentTile))
        (Variables|Default|SetCurrentTile (Variables|Default|GetTargetTile))
        (bind _output_get (Variables|Default|SetTargetTile (Default|GetNextTile (Variables|Default|GetTemp) self)))
        (Utilities|IsValid _output_get
          (:Is%20Valid
            (if (Utilities|Enum|Equal(Enum) (Variables|/Game/Blueprints/Tile.Tile_C|GetTileType (Variables|Default|GetTargetTile)) "NewEnumerator0")
              (CallFunction|MovetoTile (Variables|Default|GetTargetTile))
              (else
                (Variables|Default|SetTargetTile 0)))))))))

(event Custom|RotateToDirection
  (params (TargetRotation :type Direction%20Object%20Reference))
  (Utilities|IsValid TargetRotation
    (:Is%20Valid
      (Variables|Default|SetTargetDirection TargetRotation)
      (bind _progress (Timeline|RotateTimeline PlayFromStart)
        (:Update
          (Transformation|SetActorRotation (Math|Rotator|Lerp(Rotator) (Variables|/Game/Blueprints/Direction.Direction_C|GetRotation (Variables|Default|GetCurrentDirection)) (Variables|/Game/Blueprints/Direction.Direction_C|GetRotation (Variables|Default|GetTargetDirection)) _progress true)))
        (:Finished
          (Variables|Default|SetCurrentDirection (Variables|Default|GetTargetDirection))
          (Variables|Default|SetTargetDirection 0))))))

(event Input|ActionEvents|InputActionMoveTileUp
  (params (Key :type Key%20Structure :default "None"))
  (bind _currenttile (Variables|Default|GetCurrentTile))
  (bind _neighbours (Variables|/Game/Blueprints/Tile.Tile_C|GetNeighbours _currenttile))
  (bind _value (Utilities|Map|Find _neighbours "/Game/Blueprints/Up.Up"))
  (:Pressed
    (Utilities|IsValid (Variables|Default|GetTargetTile)
      (:Is%20Not%20Valid
        (Utilities|IsValid _value
          (:Is%20Valid
            (CallFunction|MovetoTile _value)
            (CallFunction|RotatetoDirection "/Game/Blueprints/Up.Up")))))))

(event Input|ActionEvents|InputActionMoveTileDown
  (params (Key :type Key%20Structure :default "None"))
  (bind _currenttile (Variables|Default|GetCurrentTile))
  (bind _neighbours (Variables|/Game/Blueprints/Tile.Tile_C|GetNeighbours _currenttile))
  (bind _value (Utilities|Map|Find _neighbours "/Game/Blueprints/Down.Down"))
  (:Pressed
    (Utilities|IsValid (Variables|Default|GetTargetTile)
      (:Is%20Not%20Valid
        (Utilities|IsValid _value
          (:Is%20Valid
            (CallFunction|MovetoTile _value)
            (CallFunction|RotatetoDirection "/Game/Blueprints/Down.Down")))))))

(event Input|ActionEvents|InputActionMoveTileLeft
  (params (Key :type Key%20Structure :default "None"))
  (bind _currenttile (Variables|Default|GetCurrentTile))
  (bind _neighbours (Variables|/Game/Blueprints/Tile.Tile_C|GetNeighbours _currenttile))
  (bind _value (Utilities|Map|Find _neighbours "/Game/Blueprints/Left.Left"))
  (:Pressed
    (Utilities|IsValid (Variables|Default|GetTargetTile)
      (:Is%20Not%20Valid
        (Utilities|IsValid _value
          (:Is%20Valid
            (CallFunction|MovetoTile _value)
            (CallFunction|RotatetoDirection "/Game/Blueprints/Left.Left")))))))

(event Input|ActionEvents|InputActionMoveTileRight
  (params (Key :type Key%20Structure :default "None"))
  (bind _currenttile (Variables|Default|GetCurrentTile))
  (bind _neighbours (Variables|/Game/Blueprints/Tile.Tile_C|GetNeighbours _currenttile))
  (bind _value (Utilities|Map|Find _neighbours "/Game/Blueprints/Right.Right"))
  (:Pressed
    (Utilities|IsValid (Variables|Default|GetTargetTile)
      (:Is%20Not%20Valid
        (Utilities|IsValid _value
          (:Is%20Valid
            (CallFunction|MovetoTile _value)
            (CallFunction|RotatetoDirection "/Game/Blueprints/Right.Right")))))))

(fn ConstructionScript)