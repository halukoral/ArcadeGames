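; Tile map actor that owns a Width by Height grid of Tile actors and places the player pawn on a fixed starting tile at BeginPlay.
; ResetMap destroys and respawns the grid, gives border tiles a separate type, toggles each tile's block, then has all tiles find their neighbours.
; Helpers convert between coordinates and row-major indices for lookup; IsCoordValid checks X against Height and Y against Width, unlike the other helpers.
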(event EventBeginPlay
  (bind _returnvalue (Game|Player|GetPlayerPawn 0))
  (bind _tile (Variables|Default|GetTile))
  (bind _output (Utilities|Array|Get(acopy) _tile 42))
  (Transformation|SetActorLocation _returnvalue (Transformation|GetActorLocation _output) false false)
  (Transformation|SetActorRotation _returnvalue)
  (bind _asplayer_pawn (Utilities|Casting|CastToPlayerPawn _returnvalue))
  (Variables|/Game/Blueprints/PlayerPawn.PlayerPawn_C|SetCurrentTile _asplayer_pawn _output))

(fn ConstructionScript)

(fn CoordtoIndex
  (params (Corrdinate :type Coordinate%20Structure))
  (return (+ (.x Corrdinate) (* (.y Corrdinate) (Variables|Default|GetWidth)))))

(fn IndextoCoord
  (params (Index :type Integer))
  (bind _width (Variables|Default|GetWidth))
  (return (Utilities|Struct|MakeCoordinate (Math|Integer|%(Integer) Index _width) (/ Index _width))))

(fn ResetMap
  (bind _tile (Variables|Default|GetTile))
  (bind _tilesize (Variables|Default|GetTileSize))
  (for _array_element _tile
    (Utilities|IsValid _array_element
      (:Is%20Valid
        (Actor|DestroyActor _array_element))))
  (Utilities|Array|Clear _tile)
  (for _index (range 0 (- (Variables|Default|GetHeight) 1))
    (for _index_2 (range 0 (- (Variables|Default|GetWidth) 1))
      (bind _returnvalue (Game|SpawnActorfromClass "/Game/Blueprints/Tile.Tile_C" (Math|Transform|MakeTransform (Math|Vector|MakeVector (* _index _tilesize) (* _index_2 _tilesize) 0.0) "0, 0, 0" "1,1,1") "Undefined" 0 (Utilities|Struct|MakeCoordinate _index_2 _index) (select (CallFunction|IsCoordonBorder (Utilities|Struct|MakeCoordinate _index_2 _index)) "NewEnumerator1" "NewEnumerator0") self 0))
      (Default|ToggleBlock _returnvalue)
      (Utilities|Array|Add (Variables|Default|GetTile) _returnvalue)))
  (for _array_element_2 (Variables|Default|GetTile)
    (Default|FindNeighbours _array_element_2)))

(fn IsCoordonBorder
  (params (Coord :type Coordinate%20Structure))
  (return (Math|Boolean|ORBoolean (== (.x Coord) 0) (== (.x Coord) (- (Variables|Default|GetWidth) 1)) (== (.y Coord) 0) (== (.y Coord) (- (Variables|Default|GetHeight) 1)))))

(fn IsCoordValid
  (params (Cood :type Coordinate%20Structure))
  (return (not (Math|Boolean|ORBoolean (< (.x Cood) 0) (< (.y Cood) 0) (>= (.y Cood) (Variables|Default|GetWidth)) (>= (.x Cood) (Variables|Default|GetHeight))))))

(fn GetTileatCoord
  (params (Coordinate :type Coordinate%20Structure))
  (return (Utilities|Array|Get(acopy) (Variables|Default|GetTile) (CallFunction|CoordtoIndex Coordinate))))