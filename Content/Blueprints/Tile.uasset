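; Grid tile actor that can act as a visible, solid block and links to adjacent tiles for direction-based player lookups.
; On BeginPlay, ToggleBlock enables the static mesh's collision and visibility for two tile types and disables both for all others.
; FindNeighbours uses each direction's coordinate delta to query the TileMap and cache valid tiles in a Neighbours map.
; GetNextTile returns the cached neighbour in the player's current direction.
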(event Custom|ToggleBlock
  (bind _tiletype (Variables|Default|GetTileType))
  (bind _staticmesh (Variables|Default|GetStaticMesh))
  (bind _staticmesh_2 (Variables|Default|GetStaticMesh))
  (if (or (Utilities|Enum|Equal(Enum) _tiletype "NewEnumerator1") (Utilities|Enum|Equal(Enum) _tiletype "NewEnumerator3"))
    (Collision|SetCollisionEnabled _staticmesh_2 "QueryAndPhysics")
    (Rendering|SetVisibility _staticmesh_2 true false)
    (else
      (Collision|SetCollisionEnabled _staticmesh "NoCollision")
      (Rendering|SetVisibility _staticmesh false false))))

(event EventBeginPlay
  (CallFunction|ToggleBlock))

(event Collision|EventActorBeginOverlap
  (params (OtherActor :type Actor%20Object%20Reference)))

(event EventTick
  (params (DeltaSeconds :type Float%20%28single-precision%29)))

(fn ConstructionScript)

(fn FindNeighbours
  (bind _coordinate (Variables|Default|GetCoordinate))
  (for _array_element (Utilities|Array|MakeArray "/Game/Blueprints/Up.Up" "/Game/Blueprints/Down.Down" "/Game/Blueprints/Left.Left" "/Game/Blueprints/Right.Right")
    (if (Default|IsCoordValid (Variables|Default|GetTileMap) (Utilities|Struct|MakeCoordinate (+ (.x (Variables|/Game/Blueprints/Direction.Direction_C|GetDelta _array_element)) (.x _coordinate)) (+ (.y (Variables|/Game/Blueprints/Direction.Direction_C|GetDelta _array_element)) (.y _coordinate))))
      (Utilities|IsValid (Default|GetTileatCoord (Variables|Default|GetTileMap) (Utilities|Struct|MakeCoordinate (+ (.x (Variables|/Game/Blueprints/Direction.Direction_C|GetDelta _array_element)) (.x _coordinate)) (+ (.y (Variables|/Game/Blueprints/Direction.Direction_C|GetDelta _array_element)) (.y _coordinate))))
        (:Is%20Valid
          (Utilities|Map|Add (Variables|Default|GetNeighbours) _array_element (Default|GetTileatCoord (Variables|Default|GetTileMap) (Utilities|Struct|MakeCoordinate (+ (.x (Variables|/Game/Blueprints/Direction.Direction_C|GetDelta _array_element)) (.x _coordinate)) (+ (.y (Variables|/Game/Blueprints/Direction.Direction_C|GetDelta _array_element)) (.y _coordinate))))))))))

(fn GetNextTile
  (params (PLayer :type Player%20Pawn%20Object%20Reference))
  (bind _currentdirection (Variables|/Game/Blueprints/PlayerPawn.PlayerPawn_C|GetCurrentDirection PLayer))
  (bind _neighbours (Variables|Default|GetNeighbours))
  (bind _value (Utilities|Map|Find _neighbours _currentdirection))
  (Utilities|IsValid _value
    (:Is%20Valid
      (return _value))))